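; BP_Player is a player Blueprint that moves in the Y-Z plane from Enhanced Input axes.
; BeginPlay adds the IMC_PlayerInput mapping context, and the IA_Horizontal and IA_Vertical events store their values on trigger and completion.
; Tick adds those values directly to the actor location without sweep, speed or delta-time scaling, so movement is frame-rate dependent and ignores collision blocking.
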(event Input|EnhancedActionEvents|EnhancedInputActionIA_Horizontal
  (params (ActionValue :type Float%20%28double-precision%29) (ElapsedSeconds :type Float%20%28double-precision%29) (TriggeredSeconds :type Float%20%28double-precision%29) (InputAction :type Input%20Action%20Object%20Reference :default "/Game/Inputs/IA_Horizontal.IA_Horizontal"))
  ;[1 1 1] Horizontal
  (:Triggered
    (Variables|Default|SetHorisontal ActionValue))
  (:Completed
    (Variables|Default|SetHorisontal ActionValue)))

(event Input|EnhancedActionEvents|EnhancedInputActionIA_Vertical
  (params (ActionValue :type Float%20%28double-precision%29) (ElapsedSeconds :type Float%20%28double-precision%29) (TriggeredSeconds :type Float%20%28double-precision%29) (InputAction :type Input%20Action%20Object%20Reference :default "/Game/Inputs/IA_Vertical.IA_Vertical"))
  ;[1 1 1] Vertical
  (:Triggered
    (bind _output_get (Variables|Default|SetVertical ActionValue))
    (Development|PrintString (Utilities|String|ToString(Float) _output_get)))
  (:Completed
    (Variables|Default|SetVertical ActionValue)))

(event EventBeginPlay
  ;[1 1 1] 사용자 입력 바인딩
  (Input|AddMappingContext (PlayerController|LocalPlayerSubsystems|GetEnhancedInputLocalPlayerSubsystem (Game|GetPlayerController 0)) "/Game/Inputs/IMC_PlayerInput.IMC_PlayerInput" 0 "(bIgnoreAllPressedKeysUntilRelease=True,bForceImmediately=False,bNotifyUserSettings=False)"))

(event Collision|EventActorBeginOverlap
  (params (OtherActor :type Actor%20Object%20Reference)))

(event EventTick
  (params (DeltaSeconds :type Float%20%28single-precision%29))
  (Transformation|SetActorLocation (+ (Transformation|GetActorLocation) (Math|Vector|MakeVector 0.0 (Variables|Default|GetHorisontal) (Variables|Default|GetVertical))) false false))

(fn ConstructionScript)